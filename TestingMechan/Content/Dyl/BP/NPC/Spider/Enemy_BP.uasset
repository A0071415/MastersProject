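; Spider enemy NPC that wanders to random reachable points and chases any pawn its PawnSensing spots.
; A retriggerable delay returns it to slower roaming once sightings stop, and a Disabled event temporarily knocks out its sight and movement.
; Player overlap on DestroyBox launches the player upward, then spins and destroys the spider.
; Player overlap on the attack box only pulses an attack flag; knockback and shrink logic are unwired.
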(event OnSeePawn(PawnSensing)
  (params (Pawn :type Pawn%20Object%20Reference))
  (bind _charactermovement (Variables|Character|GetCharacterMovement))
  (Utilities|FlowControl|Sequence
    (:then_0
      (Variables|/Script/Engine.CharacterMovementComponent|SetMaxWalkSpeed _charactermovement 2e+02)
      (Variables|Default|SetSpottedPlayer? true)
      (AI|AIMoveTo self "0, 0, 0" Pawn 5.0 false))
    (:then_1
      (Utilities|FlowControl|RetriggerableDelay 1.0)
      (CallFunction|RandomRoam)
      (Variables|Default|SetSpottedPlayer? false)
      (Variables|/Script/Engine.CharacterMovementComponent|SetMaxWalkSpeed _charactermovement 1.3e+02))))

(event OnComponentBeginOverlap(DestroyBox)
  (params (OverlappedComponent :type Primitive%20Component%20Object%20Reference) (OtherActor :type Actor%20Object%20Reference) (OtherComp :type Primitive%20Component%20Object%20Reference) (OtherBodyIndex :type Integer) (bFromSweep :type Boolean) (SweepResult :type Hit%20Result%20Structure%20%28by%20ref%29))
  (bind _rotatingmovement (Variables|Default|GetRotatingMovement))
  (bind _asbp_player (Utilities|Casting|CastToBP_Player OtherActor))
  (Character|LaunchCharacter _asbp_player "0.000000,0.000000,1000.000000" false true)
  (Variables|Default|SetDead? true)
  (Components|Activation|Activate _rotatingmovement false)
  (Utilities|FlowControl|Delay 1.2)
  (Components|Activation|Deactivate _rotatingmovement)
  (Utilities|FlowControl|Delay 0.5)
  (Actor|DestroyActor))

(event OnComponentBeginOverlap(Enemy_AttackBox)
  (params (OverlappedComponent :type Primitive%20Component%20Object%20Reference) (OtherActor :type Actor%20Object%20Reference) (OtherComp :type Primitive%20Component%20Object%20Reference) (OtherBodyIndex :type Integer) (bFromSweep :type Boolean) (SweepResult :type Hit%20Result%20Structure%20%28by%20ref%29))
  (bind _asbp_player (Utilities|Casting|CastToBP_Player OtherActor))
  (Utilities|FlowControl|DoOnce false :!label _label
    (:Completed
      (Variables|Default|SetAttackplayer? true)
      (Utilities|FlowControl|Delay 1.0)
      (Variables|Default|SetAttackplayer? false)
      (goto _label Reset))))

(event Custom|Random%20Roam
  (if (not (Variables|Default|GetKnockedout?))
    (AI|AIMoveTo self (.RandomLocation (AI|Navigation|GetRandomReachablePointinRadius (Transformation|GetActorLocation) 1.5e+03 0 0)) 0 5.0 false
      (:OnSuccess
        (CallFunction|RandomRoam)))))

(event Custom|Disabled
  (Variables|Default|SetKnockedout? true)
  (Variables|/Script/AIModule.PawnSensingComponent|SetSightRadius (Variables|Default|GetPawnSensing) 0.0)
  (Pawn|Components|CharacterMovement|DisableMovement (Variables|Character|GetCharacterMovement))
  (Utilities|FlowControl|Delay 5.0)
  (Variables|/Script/AIModule.PawnSensingComponent|SetSightRadius (Variables|Default|GetPawnSensing) (Variables|Default|GetDefualt%20Sight%20Radius))
  (Pawn|Components|CharacterMovement|SetMovementMode (Variables|Character|GetCharacterMovement) "MOVE_Walking" 0)
  (Variables|Default|SetKnockedout? false)
  (CallFunction|RandomRoam))

(event EventBeginPlay
  (CallFunction|RandomRoam))

(fn ConstructionScript)