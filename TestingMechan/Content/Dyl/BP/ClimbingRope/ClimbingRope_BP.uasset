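; Climbable rope actor that lets the player latch on and move in flying mode while inside its box.
; The construction script builds the rope from spline mesh segments between consecutive spline points.
; On box overlap, the player from the game instance is flagged OnRope, stopped, freed of gravity and snapped to the closest spline location.
; Leaving the box restores walking and default gravity, then launches the player upward.
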(event OnComponentBeginOverlap(Box)
  (params (OverlappedComponent :type Primitive%20Component%20Object%20Reference) (OtherActor :type Actor%20Object%20Reference) (OtherComp :type Primitive%20Component%20Object%20Reference) (OtherBodyIndex :type Integer) (bFromSweep :type Boolean) (SweepResult :type Hit%20Result%20Structure%20%28by%20ref%29))
  (bind _as_masters_p_gi (Variables|Default|GetAs%20Masters%20P%20GI))
  (bind _player (Variables|/Game/Dyl/MastersP_GI.MastersP_GI_C|GetPlayer _as_masters_p_gi))
  (bind _charactermovement (Variables|/Script/Engine.Character|GetCharacterMovement _player))
  (if (== OtherActor _player)
    (Variables|/Game/Dyl/Player/BP_Player.BP_Player_C|SetOnRope? _player true)
    (Pawn|Components|CharacterMovement|SetMovementMode _charactermovement "MOVE_Flying" 0)
    (Components|Movement|StopMovementImmediately _charactermovement)
    (Variables|/Script/Engine.CharacterMovementComponent|SetGravityScale _charactermovement 0.0)
    (Transformation|SetActorLocation _player (Spline|FindLocationClosesttoWorldLocation (Variables|Default|GetSpline) (Transformation|GetActorLocation _player) "World") false false)))

(event OnComponentEndOverlap(Box)
  (params (OverlappedComponent :type Primitive%20Component%20Object%20Reference) (OtherActor :type Actor%20Object%20Reference) (OtherComp :type Primitive%20Component%20Object%20Reference) (OtherBodyIndex :type Integer))
  (bind _as_masters_p_gi (Variables|Default|GetAs%20Masters%20P%20GI))
  (bind _player (Variables|/Game/Dyl/MastersP_GI.MastersP_GI_C|GetPlayer _as_masters_p_gi))
  (bind _charactermovement (Variables|/Script/Engine.Character|GetCharacterMovement _player))
  (if (== OtherActor _player)
    (Variables|/Game/Dyl/Player/BP_Player.BP_Player_C|SetOnRope? _player false)
    (Pawn|Components|CharacterMovement|SetMovementMode _charactermovement "MOVE_Walking" 0)
    (Variables|/Script/Engine.CharacterMovementComponent|SetGravityScale _charactermovement (Variables|/Game/Dyl/Player/BP_Player.BP_Player_C|GetDefaultGravity _player))
    (Character|LaunchCharacter _player "0.000000,0.000000,500.000000" false false)))

(event EventBeginPlay
  (bind _asmasters_p_gi (Utilities|Casting|CastToMastersP_GI (Game|GetGameInstance)))
  (Variables|Default|SetAs%20Masters%20P%20GI _asmasters_p_gi))

(fn ConstructionScript
  (bind _spline (Variables|Default|GetSpline))
  (for _index (range 0 (- (Spline|GetNumberOfSplinePoints (Variables|Default|GetSpline)) 2))
    (bind _returnvalue (AddComponent|AddSplineMeshComponent false))
    (SplineMesh|SetStartandEnd _returnvalue (.Location (Spline|GetLocationandTangentatSplinePoint _spline _index "Local")) (.Tangent (Spline|GetLocationandTangentatSplinePoint _spline _index "Local")) (.Location (Spline|GetLocationandTangentatSplinePoint _spline (+ _index 1) "Local")) (.Tangent (Spline|GetLocationandTangentatSplinePoint _spline (+ _index 1) "Local")) true :!class /Script/Engine.SplineMeshComponent)
    (Transformation|AttachComponentToComponent _returnvalue (Variables|Default|GetDefaultSceneRoot) "None" "SnapToTarget" "SnapToTarget" "SnapToTarget" true)))