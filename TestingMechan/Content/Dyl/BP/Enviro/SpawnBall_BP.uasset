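; SpawnBall_BP is an interactable that resets the ball by replacing the Ball_BP in the level.
; When the player stored in MastersP_GI overlaps its Box, it binds Interacted to that player's interact event, with no unbinding on exit.
; Interacted destroys the first Ball_BP found, waits briefly, then spawns a new one at a hard-coded location, ignoring collisions.
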(event OnComponentBeginOverlap(Box)
  (params (OverlappedComponent :type Primitive%20Component%20Object%20Reference) (OtherActor :type Actor%20Object%20Reference) (OtherComp :type Primitive%20Component%20Object%20Reference) (OtherBodyIndex :type Integer) (bFromSweep :type Boolean) (SweepResult :type Hit%20Result%20Structure%20%28by%20ref%29))
  (bind _as_masters_p_gi (Variables|Default|GetAs%20Masters%20P%20GI))
  (bind _player (Variables|/Game/Dyl/MastersP_GI.MastersP_GI_C|GetPlayer _as_masters_p_gi))
  (if (== _player OtherActor)
    (EventDispatchers|BindEventtoInteract _player (delegate Custom|Interacted))))

(event Custom|Interacted
  (bind _returnvalue (Actor|GetActorOfClass "/Game/Dyl/BP/Interactables/Ball_BP.Ball_BP_C"))
  (Actor|DestroyActor _returnvalue)
  (Utilities|FlowControl|Delay 0.1)
  (Game|SpawnActorfromClass "/Game/Dyl/BP/Interactables/Ball_BP.Ball_BP_C" (Math|Transform|MakeTransform "3261.587738,36793.155135,350.379086" "0, 0, 0" "1.000000,1.000000,1.000000") "AlwaysSpawn" "MultiplyWithRoot" 0 0))

(event EventBeginPlay
  (bind _asmasters_p_gi (Utilities|Casting|CastToMastersP_GI (Game|GetGameInstance)))
  (Variables|Default|SetAs%20Masters%20P%20GI _asmasters_p_gi))

(fn ConstructionScript)