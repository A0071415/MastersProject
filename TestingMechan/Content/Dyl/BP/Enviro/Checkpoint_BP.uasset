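; Checkpoint actor that updates the player's respawn point when the player enters its box trigger.
; On BeginPlay it caches the MastersP game instance, which holds the player reference.
; When that player overlaps the box, it stores the player's current location and rotation, with unit scale, as the SpawnTransform on the MastersP game mode.
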(event OnComponentBeginOverlap(Box)
  (params (OverlappedComponent :type Primitive%20Component%20Object%20Reference) (OtherActor :type Actor%20Object%20Reference) (OtherComp :type Primitive%20Component%20Object%20Reference) (OtherBodyIndex :type Integer) (bFromSweep :type Boolean) (SweepResult :type Hit%20Result%20Structure%20%28by%20ref%29))
  (bind _as_masters_p_gi (Variables|Default|GetAs%20Masters%20P%20GI))
  (bind _player (Variables|/Game/Dyl/MastersP_GI.MastersP_GI_C|GetPlayer _as_masters_p_gi))
  (bind _returnvalue (Transformation|GetActorTransform _player))
  (if (== _player OtherActor)
    (bind _asmasters_p_gm (Utilities|Casting|CastToMastersP_GM (Game|GetGameMode)))
    (Variables|/Game/Dyl/MastersP_GM.MastersP_GM_C|SetSpawn%20Transform _asmasters_p_gm (Math|Transform|MakeTransform (.location _returnvalue) (.rotation _returnvalue) "1.000000,1.000000,1.000000"))))

(event EventBeginPlay
  (bind _asmasters_p_gi (Utilities|Casting|CastToMastersP_GI (Game|GetGameInstance)))
  (Variables|Default|SetAs%20Masters%20P%20GI _asmasters_p_gi))

(fn ConstructionScript)