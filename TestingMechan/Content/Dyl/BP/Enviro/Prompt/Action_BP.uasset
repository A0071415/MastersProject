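; Action prompt actor that shows two text labels while the player stands inside its trigger box.
; On BeginPlay it caches the MastersP_GI game instance.
; Box overlap begin and end compare the other actor to the Player stored in that instance and toggle both TextRender components visible or hidden.
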(event OnComponentBeginOverlap(Box)
  (params (OverlappedComponent :type Primitive%20Component%20Object%20Reference) (OtherActor :type Actor%20Object%20Reference) (OtherComp :type Primitive%20Component%20Object%20Reference) (OtherBodyIndex :type Integer) (bFromSweep :type Boolean) (SweepResult :type Hit%20Result%20Structure%20%28by%20ref%29))
  (if (== (Variables|/Game/Dyl/MastersP_GI.MastersP_GI_C|GetPlayer (Variables|Default|GetAs%20Masters%20P%20GI)) OtherActor)
    (Rendering|SetVisibility (Variables|Default|GetTextRender1) true false)
    (Rendering|SetVisibility (Variables|Default|GetTextRender) true false)))

(event OnComponentEndOverlap(Box)
  (params (OverlappedComponent :type Primitive%20Component%20Object%20Reference) (OtherActor :type Actor%20Object%20Reference) (OtherComp :type Primitive%20Component%20Object%20Reference) (OtherBodyIndex :type Integer))
  (if (== (Variables|/Game/Dyl/MastersP_GI.MastersP_GI_C|GetPlayer (Variables|Default|GetAs%20Masters%20P%20GI)) OtherActor)
    (Rendering|SetVisibility (Variables|Default|GetTextRender1) false false)
    (Rendering|SetVisibility (Variables|Default|GetTextRender) false false)))

(event Collision|EventActorBeginOverlap
  (params (OtherActor :type Actor%20Object%20Reference)))

(event EventTick
  (params (DeltaSeconds :type Float%20%28single-precision%29)))

(event EventBeginPlay
  (bind _asmasters_p_gi (Utilities|Casting|CastToMastersP_GI (Game|GetGameInstance)))
  (Variables|Default|SetAs%20Masters%20P%20GI _asmasters_p_gi))

(fn ConstructionScript)