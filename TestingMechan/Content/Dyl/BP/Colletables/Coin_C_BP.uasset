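; Coin collectible actor that reports a pickup to the HUD when the player touches it.
; Its Sphere overlap compares the other actor to the Player held in the AsMastersPGI reference, then calls CoinCollected on that object's HUD.
; The actor-level overlap repeats the player check but does nothing, and the graphs neither set that reference nor destroy or hide the coin.
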(event OnComponentBeginOverlap(Sphere)
  (params (OverlappedComponent :type Primitive%20Component%20Object%20Reference) (OtherActor :type Actor%20Object%20Reference) (OtherComp :type Primitive%20Component%20Object%20Reference) (OtherBodyIndex :type Integer) (bFromSweep :type Boolean) (SweepResult :type Hit%20Result%20Structure%20%28by%20ref%29))
  (bind _as_masters_p_gi (Variables|Default|GetAs%20Masters%20P%20GI))
  (if (== (Variables|/Game/Dyl/MastersP_GI.MastersP_GI_C|GetPlayer _as_masters_p_gi) OtherActor)
    (Default|CoinCollected (Variables|/Game/Dyl/MastersP_GI.MastersP_GI_C|GetHUD _as_masters_p_gi))))

(event EventBeginPlay
  (|CallParentFunction) ; This node is disabled and will not be called.\nDrag off pins to build functionality.
)

(event Collision|EventActorBeginOverlap
  (params (OtherActor :type Actor%20Object%20Reference))
  (if (== (Variables|/Game/Dyl/MastersP_GI.MastersP_GI_C|GetPlayer (Variables|Default|GetAs%20Masters%20P%20GI)) OtherActor)
    _))

(event EventTick
  (params (DeltaSeconds :type Float%20%28single-precision%29)))

(fn ConstructionScript
  (|CallParentFunction))