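; DestroyableBox_BP is an interactable box that is destroyed when it takes any damage while CanBeDestroyed is set.
; It caches the MastersP_GI game instance on BeginPlay to reach the HUD.
; On damage it increments its own IntDestroyedCounter, writes that value to the HUD's BoxesDestroyed, calls BoxDestroyed on the HUD, then destroys itself.
; The counter lives on the box rather than in the game instance.
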(event Game|Damage|EventAnyDamage
  (params (Damage :type Float%20%28single-precision%29) (DamageType :type Damage%20Type%20Object%20Reference) (InstigatedBy :type Controller%20Object%20Reference) (DamageCauser :type Actor%20Object%20Reference))
  (if (Variables|Default|GetCanBeDestroyed?)
    (bind _result (Math|Integer|IncrementInt (Variables|Default|GetInt%20+DestroyedCounter))
      (:%20%20
        (Variables|/Game/Dyl/UI/HUD_WBP.HUD_WBP_C|SetBoxesDestroyed (Variables|/Game/Dyl/MastersP_GI.MastersP_GI_C|GetHUD (stale EventBeginPlay _asmasters_p_gi)) _result)
        (Default|BoxDestroyed (Variables|/Game/Dyl/MastersP_GI.MastersP_GI_C|GetHUD (stale EventBeginPlay _asmasters_p_gi)))
        (Actor|DestroyActor)))))

(event EventBeginPlay
  (bind _asmasters_p_gi (Utilities|Casting|CastToMastersP_GI (Game|GetGameInstance))))

(fn ConstructionScript)