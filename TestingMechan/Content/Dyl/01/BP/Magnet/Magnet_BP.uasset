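; Magnet actor that flips between red and blue polarity to move colored obstacles and gives the player a magnet on overlap.
; From BeginPlay, two events call each other endlessly, each recoloring the light, rolling the actor 180 degrees and calling MoveObject on that color's obstacles.
; The switching Delay sits inside each loop body, so an empty array halts the cycle.
; Sphere overlap reveals BP_Player's MagnetBack and sets HasMagnet.
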(event OnComponentBeginOverlap(Sphere)
  (params (OverlappedComponent :type Primitive%20Component%20Object%20Reference) (OtherActor :type Actor%20Object%20Reference) (OtherComp :type Primitive%20Component%20Object%20Reference) (OtherBodyIndex :type Integer) (bFromSweep :type Boolean) (SweepResult :type Hit%20Result%20Structure%20%28by%20ref%29))
  (bind _asbp_player (Utilities|Casting|CastToBP_Player OtherActor))
  (Development|SetHiddeninGame (Variables|/Game/Dyl/BP_Player.BP_Player_C|GetMagnetBack _asbp_player) false false)
  (Variables|/Game/Dyl/BP_Player.BP_Player_C|SetHasMagnet? _asbp_player true))

(event Custom|Changing%20To%20Red
  (bind _returnvalue (Transformation|GetActorRotation))
  (Rendering|Components|Light|SetLightColor (Variables|Default|GetPointLight) "(R=1.000000,G=0.000000,B=0.000000,A=1.000000)" true)
  (Transformation|SetActorRotation (Math|Rotator|MakeRotator (+ (.roll _returnvalue) 1.8e+02) (.pitch _returnvalue) (.yaw _returnvalue)))
  (Utilities|FlowControl|Delay 0.2)
  (for _array_element (Variables|Default|GetMoveRed_Obstacles)
    (Default|MoveObject _array_element)
    (Utilities|FlowControl|Delay 2.0)
    (CallFunction|ChangingtoBlue)))

(event Custom|Changing%20To%20Blue
  (bind _returnvalue (Transformation|GetActorRotation))
  (Rendering|Components|Light|SetLightColor (Variables|Default|GetPointLight) "(R=0.000000,G=0.652499,B=0.947917,A=1.000000)" true)
  (Transformation|SetActorRotation (Math|Rotator|MakeRotator (+ (.roll _returnvalue) 1.8e+02) (.pitch _returnvalue) (.yaw _returnvalue)))
  (Utilities|FlowControl|Delay 0.2)
  (for _array_element (Variables|Default|GetMoveBlue_Obstacles)
    (Default|MoveObject _array_element)
    (Utilities|FlowControl|Delay 2.0)
    (CallFunction|ChangingtoRed)))

(event EventBeginPlay
  (CallFunction|ChangingtoRed))

(fn ConstructionScript)