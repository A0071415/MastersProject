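; GrappleLine_BP is a zipline-style spline actor that carries the player along a cable when they overlap its box.
; The construction script builds the cable from spline mesh segments between spline points, shifted by CableOffset.
; On overlap, it disables input, flags RidingGrappleLine, aligns the player to the spline and moves them along it via a Timeline, restoring control when finished.
; MoveObject is empty, and the LastMovedFWD direction toggle is disconnected.
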(event OnComponentBeginOverlap(Box)
  (params (OverlappedComponent :type Primitive%20Component%20Object%20Reference) (OtherActor :type Actor%20Object%20Reference) (OtherComp :type Primitive%20Component%20Object%20Reference) (OtherBodyIndex :type Integer) (bFromSweep :type Boolean) (SweepResult :type Hit%20Result%20Structure%20%28by%20ref%29))
  (bind _returnvalue (Game|GetPlayerController 0))
  (bind _as_bp_player (Variables|Default|GetAs%20BP%20Player))
  (bind _spline (Variables|Default|GetSpline))
  (bind _as_bp_player_2 (Variables|Default|GetAs%20BP%20Player))
  (if (== _as_bp_player OtherActor)
    (Input|DisableInput _as_bp_player _returnvalue)
    (Variables|/Game/Dyl/BP_Player.BP_Player_C|SetRidingGrappleLine? _as_bp_player_2 true)
    (Transformation|SetActorRotation _as_bp_player (Transformation|GetWorldRotation _spline))
    (bind _newtrack_0 (Timeline|Timeline PlayFromStart)
      (:Update
        (Transformation|SetWorldLocation (Variables|/Script/Engine.Actor|GetRootComponent (Variables|Default|GetAs%20BP%20Player)) (Spline|GetLocationatTime _spline _newtrack_0 "World" false) false false))
      (:Finished
        (Variables|/Game/Dyl/BP_Player.BP_Player_C|SetRidingGrappleLine? _as_bp_player_2 false)
        (Input|EnableInput _as_bp_player _returnvalue)))))

(event Custom|MoveObject)

(event EventBeginPlay
  (bind _asbp_player (Utilities|Casting|CastToBP_Player (Game|GetPlayerCharacter 0)))
  (Variables|Default|SetAs%20BP%20Player _asbp_player))

(fn ConstructionScript
  (bind _spline (Variables|Default|GetSpline))
  (bind _cableoffset (Variables|Default|GetCableOffset))
  (for _index (range (- (Spline|GetNumberOfSplinePoints (Variables|Default|GetSpline)) 2) 0)
    (bind _returnvalue (AddComponent|AddSplineMeshComponent false))
    (SplineMesh|SetStartandEnd _returnvalue (+ (.Location (Spline|GetLocationandTangentatSplinePoint _spline _index "Local")) _cableoffset) (.Tangent (Spline|GetLocationandTangentatSplinePoint _spline _index "Local")) (+ (.Location (Spline|GetLocationandTangentatSplinePoint _spline (+ _index 1) "Local")) _cableoffset) (.Tangent (Spline|GetLocationandTangentatSplinePoint _spline (+ _index 1) "Local")) true :!class /Script/Engine.SplineMeshComponent)
    (Transformation|AttachComponentToComponent _returnvalue (Variables|Default|GetDefaultSceneRoot) "None" "SnapToTarget" "SnapToTarget" "SnapToTarget" true)))